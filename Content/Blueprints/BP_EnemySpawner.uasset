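; BP_EnemySpawner periodically spawns BP_U1EnemyE_02 enemies at random points within its SpawnableArea box.
; Tick accumulates a timer and, past SpawnDelay, resets it and rerolls a random ground-plane point until one lies outside SpawnIgnoreAreaRange of player 0, using squared distance.
; The random point is re-evaluated at each use, so the printed and spawned locations differ from the tested one and spawns can land near the player.
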(event EventBeginPlay)

(event Collision|EventActorBeginOverlap
  (params (OtherActor :type Actor%20Object%20Reference)))

(event EventTick
  (params (DeltaSeconds :type Float%20%28single-precision%29))
  (bind _spawnablearea (Variables|Default|GetSpawnableArea))
  (bind _returnvalue (Components|Box|GetScaledBoxExtent _spawnablearea))
  (bind _returnvalue_2 (Transformation|GetWorldLocation _spawnablearea))
  (bind _returnvalue_3 (Math|Random|RandomPointinBoundingBox _returnvalue_2 _returnvalue))
  (bind (_x _y) (Math|Vector|BreakVector _returnvalue_3))
  (bind _returnvalue_4 (Math|Vector|MakeVector _x _y 0.0))
  ;[1 1 1] Timer
  (bind _output_get (Variables|Spawn|SetSpawnTimer (+ DeltaSeconds (Variables|Spawn|GetSpawnTimer))))
  (if (> _output_get (Variables|Spawn|GetSpawnDelay))
    (Variables|Spawn|SetSpawnTimer 0.0 :!label _label)
    (while (< (Math|Vector|VectorLengthSquared (- _returnvalue_4 (Transformation|GetActorLocation (Game|Player|GetPlayerPawn 0)))) (* (Variables|Spawn|GetSpawnIgnoreAreaRange) (Variables|Spawn|GetSpawnIgnoreAreaRange)))
      (goto _label))
    (Development|PrintString (Utilities|String|ToString(Vector) _returnvalue_4))
    (Game|SpawnActorfromClass "/Game/Blueprints/Entity/Enemy/BP_U1EnemyE_02.BP_U1EnemyE_02_C" (Math|Transform|MakeTransform (Math|Vector|MakeVector _x _y 1e+02)) "Undefined" "MultiplyWithRoot" 0 0)))

(fn ConstructionScript)