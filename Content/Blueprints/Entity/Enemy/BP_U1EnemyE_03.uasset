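; BP_U1EnemyE_03 is an enemy Blueprint with a spinning grinder that periodically deals area damage.
; Each tick it rotates the static mesh around the up axis at GrinderRotationSpeed and advances an attack timer.
; When the timer exceeds the AttackDelay stat from StatComponent, it resets and U1SphereDamageCaster casts AttackPower damage with no knockback and popup text.
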(event EventBeginPlay)

(event Collision|EventActorBeginOverlap
  (params (OtherActor :type Actor%20Object%20Reference)))

(event EventTick
  (params (DeltaSeconds :type Float%20%28single-precision%29))
  (bind _statcomponent (Variables|Default|GetStatComponent))
  (Transformation|AddLocalRotation (Variables|Default|GetStaticMeshComponent) (Math|Vector|RotatorfromAxisandAngle (Math|Vector|VectorUp) (* DeltaSeconds (Variables|Components|GetGrinderRotationSpeed))) false false)
  (bind _output_get (Variables|Components|SetAttackTimer (+ DeltaSeconds (Variables|Components|GetAttackTimer))))
  (bind _returnvalue (Class|U1StatComponent|GetFinalStatValue _statcomponent "AttackDelay"))
  (if (> _output_get _returnvalue)
    (Variables|Components|SetAttackTimer 0.0)
    (bind _returnvalue_2 (Class|U1StatComponent|GetFinalStatIntegerValue _statcomponent "AttackPower"))
    (Class|U1DamageCaster|CastDamage (Variables|Default|GetU1SphereDamageCaster) (Utilities|Struct|MakeAttackInfo _returnvalue_2 "Default" "0.000000,0.000000,0.000000") true)))

(fn ConstructionScript)